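; Actor Blueprint that plays a timeline-driven motion of its Capsule0 component as soon as play begins.
; BeginPlay calls the StartShow event, which plays a timeline from the start.
; On each timeline update, the TransformCollider track value is added as a local offset to the capsule without sweeping, so the movement accumulates per update rather than setting an absolute position.
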(event EventBeginPlay
  (|CallParentFunction)
  (CallFunction|StartShow))

(event Collision|EventActorBeginOverlap
  (params (OtherActor :type Actor%20Object%20Reference))
  (|CallParentFunction OtherActor) ; This node is disabled and will not be called.\nDrag off pins to build functionality.
)

(event EventTick
  (params (DeltaSeconds :type Float%20%28single-precision%29))
  (|CallParentFunction DeltaSeconds))

(event Custom|StartShow
  (bind _transform_collider (Timeline|Timeline_0_0 PlayFromStart)
    (:Update
      (Transformation|AddLocalOffset (Variables|Default|GetCapsule_0) _transform_collider false false))))

(fn ConstructionScript
  (|CallParentFunction))